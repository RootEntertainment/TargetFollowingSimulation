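; BP_Charactor is a wandering NPC that can draw a trail of its path.
; MoveNPC sends it to a random reachable nearby point with AIMoveTo, then calls itself again after a pause, with a much shorter wait on failure.
; When ShowTrace is set, a throttled Tick draws persistent debug lines in LineColor from the last recorded location to the current one.
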(event `self.ReceiveBeginPlay`
  (`self.SetActorTickInterval` 0.2)
  (set `self.LastLocation` (`self.K2_GetActorLocation`))
  (`self.MoveNPC`))

(event `MoveNPC`
  (bind _output_get (set `self.Random Location` (`NavigationSystemV1.K2_GetRandomReachablePointInRadius` (`self.K2_GetActorLocation`) 1000.0 null null)))
  (`|AIMoveTo` self _output_get null
    (:`OnSuccess`
      (`KismetSystemLibrary.Delay` 4.0))
    (:`OnFail`
      (`KismetSystemLibrary.Delay` 0.2)))
  (`self.MoveNPC`))

(event `self.ReceiveTick`
  (params (DeltaSeconds :type "Float (single-precision)"))
  (bind _returnvalue (`self.K2_GetActorLocation`))
  (if (`self.bShowTrace`)
    (`KismetSystemLibrary.DrawPersistDebugLine` (`self.LastLocation`) _returnvalue (`self.Line Color`) true)
    (set `self.LastLocation` _returnvalue)))

(fn `UserConstructionScript`)